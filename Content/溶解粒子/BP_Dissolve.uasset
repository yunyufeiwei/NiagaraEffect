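; BP_Dissolve is an actor that plays a dissolve effect with particles on a skeletal mesh when play begins.
; A timeline drives one Dissolve_Intensity value into both the mesh materials and the Niagara component, keeping shader and particles in step.
; Each update also rebinds the skeletal mesh to the Niagara system, though the override name is left empty.
; A fixed-value copy of this logic sits unconnected in the construction script.
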(event EventBeginPlay
  (bind _dissolve_value (Timeline|Dissolve%20Value Play)
    (:Update
      (Rendering|Material|SetScalarParameterValueonMaterials (Variables|Default|GetSkeletalMesh) "Dissolve_Intensity" _dissolve_value)
      (Class|NiagaraFunctionLibrary|OverrideSystemUserVariableSkeletalMeshComponent (Variables|Default|GetNiagara) "" (Variables|Default|GetSkeletalMesh))
      (Niagara|SetNiagaraVariable(Float) (Variables|Default|GetNiagara) "Dissolve_Intensity" _dissolve_value))))

(fn ConstructionScript)